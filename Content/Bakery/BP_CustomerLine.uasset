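; BP_CustomerLine runs the bakery's customer queue along a spline, from spawn through the display to exit.
; Once the bakery opens, randomized timers request customers, which spawn at the spline start while the line has room.
; Tick advances them into spaced slots behind the display point, updating BakerController world state with arrivals and the front customer's demand.
; Satisfied customers move to a leaving list, continue along the spline and are destroyed at its end.
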(event Custom|OpenBakery
  (Utilities|Time|SetTimerbyEvent (delegate Custom|AddCustomer) 5.0))

(event Custom|AddCustomer
  (Variables|Default|SetWantCustomerAdd true))

(event EventBeginPlay
  (Variables|Default|SetDisplayDistance (Spline|GetDistanceAlongSplineatSplinePoint (Variables|Default|GetLine) (Variables|Default|GetDisplayKey))))

(event EventTick
  (params (DeltaSeconds :type Float%20%28single-precision%29))
  (bind _returnvalue (Utilities|Enum|LiteralenumEnum_BakeryWorldState "NewEnumerator30"))
  (bind _bakercontroller (Variables|Default|GetBakerController))
  (CallFunction|HandleCustomers)
  (for (_array_element _array_index) (Variables|Default|GetCustomersInLine)
    (bind _output_get (Variables|/Game/Bakery/BP_Customer.BP_Customer_C|SetDistance _array_element (Math|Float|Clamp(Float) (+ (* DeltaSeconds 5e+01) (Variables|/Game/Bakery/BP_Customer.BP_Customer_C|GetDistance _array_element)) 0.0 (- (Variables|Default|GetDisplayDistance) (* _array_index 1e+02)))))
    (Transformation|SetActorLocation _array_element (Spline|GetLocationatDistanceAlongSpline (Variables|Default|GetLine) _output_get "World") false false)
    (if (and (== _output_get (- (Variables|Default|GetDisplayDistance) (* _array_index 1e+02))) (not (Variables|/Game/Bakery/BP_Customer.BP_Customer_C|GetInLine _array_element)))
      (Variables|/Game/Bakery/BP_Customer.BP_Customer_C|SetInLine _array_element true)
      (Utilities|FlowControl|Sequence
        (:then_0
          (bind _value (Class|SHTNControllerLibrary|GetWorldStateValue _bakercontroller _returnvalue))
          (Class|SHTNControllerLibrary|SetWorldStateasValue _bakercontroller _returnvalue (+ _value 1)))
        (:then_1
          (if (== (Variables|/Game/Bakery/BP_Customer.BP_Customer_C|GetDistance _array_element) (Variables|Default|GetDisplayDistance))
            (Class|SHTNControllerLibrary|SetWorldStateasValue _bakercontroller (Utilities|Enum|LiteralenumEnum_BakeryWorldState "NewEnumerator31") (Variables|/Game/Bakery/BP_Customer.BP_Customer_C|GetDemand _array_element)))))))
  (for _array_element_2 (Variables|Default|GetLeavingCustomers)
    (bind _output_get_2 (Variables|/Game/Bakery/BP_Customer.BP_Customer_C|SetDistance _array_element_2 (+ (* DeltaSeconds 5e+01) (Variables|/Game/Bakery/BP_Customer.BP_Customer_C|GetDistance _array_element_2))))
    (if (>= _output_get_2 (Spline|GetSplineLength (Variables|Default|GetLine)))
      (Actor|DestroyActor _array_element_2)
      (Utilities|Array|RemoveItem (Variables|Default|GetLeavingCustomers) _array_element_2)
      (else
        (Transformation|SetActorLocation _array_element_2 (Spline|GetLocationatDistanceAlongSpline (Variables|Default|GetLine) _output_get_2 "World") false false)))))

(fn ConstructionScript)

(fn IsCustomeratDisplay
  (return (== (Variables|/Game/Bakery/BP_Customer.BP_Customer_C|GetDistance (Utilities|Array|Get(acopy) (Variables|Default|GetCustomersInLine))) (Variables|Default|GetDisplayDistance))))

(fn SatisfyCustomer
  (Utilities|Array|Add (Variables|Default|GetLeavingCustomers) (Utilities|Array|Get(acopy) (Variables|Default|GetCustomersInLine)))
  (Utilities|Array|RemoveIndex (Variables|Default|GetCustomersInLine)))

(fn GetCustomerDemand
  (bind _customersinline (Variables|Default|GetCustomersInLine))
  (if (> (Utilities|Array|Length _customersinline) 0)
    (return (Variables|/Game/Bakery/BP_Customer.BP_Customer_C|GetDemand (Utilities|Array|Get(acopy) _customersinline)))
    (else
      (return 0))))

(fn HandleCustomers
  (if (and (Variables|Default|GetWantCustomerAdd) (< (Utilities|Array|Length (Variables|Default|GetCustomersInLine)) (Variables|Default|GetMaxCustomersInLine)))
    (Variables|Default|SetWantCustomerAdd false)
    (bind _returnvalue (Game|SpawnActorfromClass "/Game/Bakery/BP_Customer.BP_Customer_C" (Math|Transform|MakeTransform (Spline|GetLocationatSplinePoint (Variables|Default|GetLine) 0 "World") "0, 0, 0" "1,1,1") "AlwaysSpawn" 0 0))
    (Utilities|Array|Add (Variables|Default|GetCustomersInLine) _returnvalue)
    (Utilities|Time|SetTimerbyEvent (EventDispatchers|CreateEvent :!event Custom|AddCustomer) (Math|Random|RandomFloatinRange 15.0 45.0))))