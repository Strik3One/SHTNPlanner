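; AI controller for the bakery's baker agent, driven by an HTN planner running the BPN_BakerNetwork network.
; On BeginPlay it caches the first actor found of each station class and maps location enums to their interaction transforms, including the order machine's ingredients.
; The first TargetPoint found serves as the wait spot, and the controller registers itself with the customer line before starting the planner.
; On possess it stores the BP_BakerAgent pawn.
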(event EventBeginPlay
  (CallFunction|SetupLocations)
  (Class|SHTNControllerLibrary|RunHTNPlanner self "/Game/Bakery/BakerAgent/BPN_BakerNetwork.BPN_BakerNetwork_C"))

(event EventTick
  (params (DeltaSeconds :type Float%20%28single-precision%29)))

(event EventPossess
  (params (PossessedPawn :type Pawn%20Object%20Reference))
  (bind _asbp_baker_agent (Utilities|Casting|CastToBP_BakerAgent PossessedPawn))
  (Variables|Default|SetBakerAgent _asbp_baker_agent))

(fn ConstructionScript)

(fn SetupLocations
  (bind _locations (Variables|Default|GetLocations))
  (Utilities|FlowControl|Sequence
    (:then_0
      ;[1 1 1] Oven
      (bind _outactors (Actor|GetAllActorsOfClass "/Game/Bakery/Appliances/BP_Oven.BP_Oven_C"))
      (Variables|Appliances|SetOven (Utilities|Array|Get(acopy) _outactors))
      (Utilities|Map|Add (Variables|Default|GetLocations) "NewEnumerator25" (Transformation|GetWorldTransform (Variables|/Game/Bakery/Appliances/BP_Oven.BP_Oven_C|GetInteractionLocation (Utilities|Array|Get(acopy) _outactors)))))
    (:then_1
      ;[1 1 1] Cooler
      (bind _outactors_2 (Actor|GetAllActorsOfClass "/Game/Bakery/Appliances/BP_RisingCooler.BP_RisingCooler_C"))
      (bind _output_get (Variables|Appliances|SetCooler (Utilities|Array|Get(acopy) _outactors_2)))
      (Utilities|Map|Add (Variables|Default|GetLocations) "NewEnumerator24" (Transformation|GetWorldTransform (Variables|/Game/Bakery/Appliances/BP_RisingCooler.BP_RisingCooler_C|GetInteractionLocation _output_get))))
    (:then_2
      ;[1 1 1] WaitLocation
      (bind _outactors_3 (Actor|GetAllActorsOfClass "/Script/Engine.TargetPoint"))
      (Utilities|Map|Add (Variables|Default|GetLocations) "NewEnumerator22" (Transformation|GetActorTransform (Utilities|Array|Get(acopy) _outactors_3))))
    (:then_3
      ;[1 1 1] Mixer
      (bind _outactors_4 (Actor|GetAllActorsOfClass "/Game/Bakery/Appliances/BP_Mixer.BP_Mixer_C"))
      (Variables|Appliances|SetMixer (Utilities|Array|Get(acopy) _outactors_4))
      (Utilities|Map|Add (Variables|Default|GetLocations) "NewEnumerator23" (Transformation|GetWorldTransform (Variables|/Game/Bakery/Appliances/BP_Mixer.BP_Mixer_C|GetInteractionLocation (Utilities|Array|Get(acopy) _outactors_4)))))
    (:then_4
      ;[1 1 1] CoolingTable
      (bind _outactors_5 (Actor|GetAllActorsOfClass "/Game/Bakery/Appliances/BP_CoolingTable.BP_CoolingTable_C"))
      (Variables|Appliances|SetCoolingTable (Utilities|Array|Get(acopy) _outactors_5))
      (Utilities|Map|Add (Variables|Default|GetLocations) "NewEnumerator26" (Transformation|GetWorldTransform (Variables|/Game/Bakery/Appliances/BP_CoolingTable.BP_CoolingTable_C|GetInteractionLocation (Utilities|Array|Get(acopy) _outactors_5)))))
    (:then_5
      ;[1 1 1] Display
      (bind _outactors_6 (Actor|GetAllActorsOfClass "/Game/Bakery/Appliances/BP_Display.BP_Display_C"))
      (Variables|Appliances|SetDisplay (Utilities|Array|Get(acopy) _outactors_6))
      (Utilities|Map|Add (Variables|Default|GetLocations) "NewEnumerator27" (Transformation|GetWorldTransform (Variables|/Game/Bakery/Appliances/BP_Display.BP_Display_C|GetInteractionLocation (Utilities|Array|Get(acopy) _outactors_6)))))
    (:then_6
      ;[1 1 1] DoughTable
      (bind _outactors_7 (Actor|GetAllActorsOfClass "/Game/Bakery/Appliances/BP_DoughTable.BP_DoughTable_C"))
      (Variables|Appliances|SetDoughTable (Utilities|Array|Get(acopy) _outactors_7))
      (Utilities|Map|Add (Variables|Default|GetLocations) "NewEnumerator28" (Transformation|GetWorldTransform (Variables|/Game/Bakery/Appliances/BP_DoughTable.BP_DoughTable_C|GetInteractionLocation (Utilities|Array|Get(acopy) _outactors_7)))))
    (:then_7
      ;[1 1 1] OrderMachine and Ingredients
      (bind _outactors_8 (Actor|GetAllActorsOfClass "/Game/Bakery/Appliances/BP_OrderMachine.BP_OrderMachine_C"))
      (Variables|Appliances|SetOrderMachine (Utilities|Array|Get(acopy) _outactors_8))
      (Utilities|Map|Add _locations "NewEnumerator29" (Transformation|GetWorldTransform (Variables|/Game/Bakery/Appliances/BP_OrderMachine.BP_OrderMachine_C|GetInteractionLocation (Utilities|Array|Get(acopy) _outactors_8))))
      (Utilities|Map|Add _locations "NewEnumerator18" (Transformation|GetWorldTransform (Variables|/Game/Bakery/Appliances/BP_OrderPallet.BP_OrderPallet_C|GetInteractionLocation (Variables|/Game/Bakery/Appliances/BP_OrderMachine.BP_OrderMachine_C|GetFlour (Utilities|Array|Get(acopy) _outactors_8)))))
      (Utilities|Map|Add _locations "NewEnumerator20" (Transformation|GetWorldTransform (Variables|/Game/Bakery/Appliances/BP_OrderPallet.BP_OrderPallet_C|GetInteractionLocation (Variables|/Game/Bakery/Appliances/BP_OrderMachine.BP_OrderMachine_C|GetYeast (Utilities|Array|Get(acopy) _outactors_8)))))
      (Utilities|Map|Add _locations "NewEnumerator19" (Transformation|GetWorldTransform (Variables|/Game/Bakery/Appliances/BP_OrderPallet.BP_OrderPallet_C|GetInteractionLocation (Variables|/Game/Bakery/Appliances/BP_OrderMachine.BP_OrderMachine_C|GetSalt (Utilities|Array|Get(acopy) _outactors_8))))))
    (:then_8
      (bind _outactors_9 (Actor|GetAllActorsOfClass "/Game/Bakery/BP_CustomerLine.BP_CustomerLine_C"))
      (bind _output_get_2 (Variables|Default|SetCustomerLine (Utilities|Array|Get(acopy) _outactors_9)))
      (Variables|/Game/Bakery/BP_CustomerLine.BP_CustomerLine_C|SetBakerController _output_get_2 self))))