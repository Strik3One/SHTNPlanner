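; BP_OrderPallet is a bakery appliance representing a pallet that holds stock of one ingredient type.
; SetIngredientType stores the type and shows its name on a text label.
; Restock refills Fullness to 100, while Grab subtracts the requested amount.
; Tick smoothly interpolates the product mesh's vertical scale toward the Fullness percentage, clamped so it never fully flattens.
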(event EventBeginPlay)

(event Collision|EventActorBeginOverlap
  (params (OtherActor :type Actor%20Object%20Reference)))

(event EventTick
  (params (DeltaSeconds :type Float%20%28single-precision%29))
  (Transformation|SetRelativeScale3D (Variables|Default|GetProductScale) (Math|Vector|MakeVector 1.0 1.0 (Math|Float|Clamp(Float) (Math|Interpolation|FInterpTo (.z (Variables|/Script/Engine.SceneComponent|GetRelativeScale3D (Variables|Default|GetProductScale))) (* (Variables|Default|GetFullness) 0.01) DeltaSeconds 5.0) 0.01))))

(fn ConstructionScript)

(fn SetIngredientType
  (params (Type :type Enum_IngredientTypes%20Enum :default "NewEnumerator0"))
  (bind _output_get (Variables|Default|SetIngredientType Type))
  (Rendering|Components|TextRender|SetText (Variables|Default|GetIngredient) (Utilities|Text|ToText(String) (Utilities|String|EnumtoString _output_get))))

(fn Restock
  (Variables|Default|SetFullness 100))

(fn Grab
  (params (Amount :type Integer))
  (Variables|Default|SetFullness (- (Variables|Default|GetFullness) Amount)))