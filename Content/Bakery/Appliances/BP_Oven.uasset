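; BP_Oven is a bakery oven that runs a timed bake for a Baker.
; StartOven stores the Baker, turns on the light and smoke, closes the door and starts a fixed timer.
; When the timer fires, it changes the tray's state, stops the effects, updates two world-state keys on the Baker and opens the door.
; Tick slides the door vertically at constant speed toward its open or closed position.
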(event Custom|StartOven
  (params (Baker :type PC%20Baker%20Controller%20Object%20Reference))
  (Variables|Default|SetBakerController Baker)
  (Rendering|SetVisibility (Variables|Default|GetOvenLight) true false)
  (Components|Activation|Activate (Variables|Default|GetSmoke) false)
  (Variables|Default|SetOpen false)
  (Utilities|Time|SetTimerbyEvent (delegate Custom|FinishOven) 3e+01))

(event Custom|FinishOven
  (Default|SetTrayState (Variables|Default|GetTray) "NewEnumerator2")
  (Rendering|SetVisibility (Variables|Default|GetOvenLight) false false)
  (Components|Activation|Deactivate (Variables|Default|GetSmoke))
  (Class|SHTNControllerLibrary|SetWorldStateasValue (Variables|Default|GetBakerController) (Utilities|Enum|LiteralenumEnum_BakeryWorldState "NewEnumerator7") 1)
  (Class|SHTNControllerLibrary|SetWorldStateasValue (Variables|Default|GetBakerController) (Utilities|Enum|LiteralenumEnum_BakeryWorldState "NewEnumerator8"))
  (Variables|Default|SetOpen true))

(event EventBeginPlay)

(event Collision|EventActorBeginOverlap
  (params (OtherActor :type Actor%20Object%20Reference)))

(event EventTick
  (params (DeltaSeconds :type Float%20%28single-precision%29))
  (bind _ovendoor (Variables|Default|GetOvenDoor))
  (Transformation|SetRelativeLocation _ovendoor (Math|Interpolation|VInterptoConstant (Variables|/Script/Engine.SceneComponent|GetRelativeLocation _ovendoor) (select (Variables|Default|GetOpen) "45.000000, 0,70.000000" "45.000000,0.000000,130.000000") DeltaSeconds 4e+01) false false))

(fn ConstructionScript)