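; BP_Display is a bakery display that shows its bread stock through 18 bread components, gathered into an array by the construction script.
; AddBread increments the count and reveals the matching bread; the first ever added also finds the BP_CustomerLine and opens the bakery.
; RemoveBread lowers the count and hides the freed top slots, with no bounds checks in either direction.
; Removebreadtest is a test wrapper for removal.
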(event EventBeginPlay)

(event Collision|EventActorBeginOverlap
  (params (OtherActor :type Actor%20Object%20Reference)))

(event EventTick
  (params (DeltaSeconds :type Float%20%28single-precision%29)))

(fn ConstructionScript
  (Variables|Default|SetBreadsArray (Utilities|Array|MakeArray (Variables|Default|GetBread1) (Variables|Default|GetBread2) (Variables|Default|GetBread3) (Variables|Default|GetBread4) (Variables|Default|GetBread5) (Variables|Default|GetBread6) (Variables|Default|GetBread7) (Variables|Default|GetBread8) (Variables|Default|GetBread9) (Variables|Default|GetBread10) (Variables|Default|GetBread11) (Variables|Default|GetBread12) (Variables|Default|GetBread13) (Variables|Default|GetBread14) (Variables|Default|GetBread15) (Variables|Default|GetBread16) (Variables|Default|GetBread17) (Variables|Default|GetBread18))))

(fn AddBread
  (bind _result (Math|Integer|IncrementInt (Variables|Default|GetBreads))
    (:%20%20
      (Rendering|SetVisibility (Utilities|Array|Get(acopy) (Variables|Default|GetBreadsArray) (- _result 1)) true true)
      (if (not (Variables|Default|GetFirstBread))
        (Variables|Default|SetFirstBread true)
        (bind _outactors (Actor|GetAllActorsOfClass "/Game/Bakery/BP_CustomerLine.BP_CustomerLine_C"))
        (Default|OpenBakery (Utilities|Array|Get(acopy) _outactors))))))

(fn RemoveBread
  (params (Amount :type Integer))
  (Variables|Default|SetBreads (- (Variables|Default|GetBreads) Amount))
  (for _index (range 0 (- Amount 1))
    (Rendering|SetVisibility (Utilities|Array|Get(acopy) (Variables|Default|GetBreadsArray) (+ _index (Variables|Default|GetBreads))) false false)))

(fn Removebreadtest
  (CallFunction|RemoveBread 2))