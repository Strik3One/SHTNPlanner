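; Bakery mixer appliance that takes flour, yeast and salt and runs a timed mix for a baker.
; AddIngredient flags each ingredient and counts them into Fullness, which Tick uses to smoothly raise or lower the fill mesh.
; StartMixer stores the baker, activates dust and clears the ingredient flags.
; When the timer ends, it swaps the fill material, stops the dust and updates two world-state values on the baker.
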(event Custom|StartMixer
  (params (Baker :type PC%20Baker%20Controller%20Object%20Reference))
  (Variables|Default|SetBakerController Baker)
  (Components|Activation|Activate (Variables|Default|GetMixerDust) false)
  (Variables|Default|SetIsFlourLoaded false)
  (Variables|Default|SetIsSaltLoaded false)
  (Variables|Default|SetIsYeastLoaded false)
  (Utilities|Time|SetTimerbyEvent (delegate Custom|FinishMixer) 15.0))

(event Custom|FinishMixer
  (bind _bakercontroller (Variables|Default|GetBakerController))
  (Rendering|Material|SetMaterial (Variables|Default|GetMixerFill) 0 "/Game/Bakery/Materials/MI_Pallet.MI_Pallet")
  (Components|Activation|Deactivate (Variables|Default|GetMixerDust))
  (Class|SHTNControllerLibrary|SetWorldStateasValue _bakercontroller (Utilities|Enum|LiteralenumEnum_BakeryWorldState "NewEnumerator13") 3)
  (Class|SHTNControllerLibrary|SetWorldStateasValue _bakercontroller (Utilities|Enum|LiteralenumEnum_BakeryWorldState "NewEnumerator17")))

(event EventBeginPlay)

(event EventTick
  (params (DeltaSeconds :type Float%20%28single-precision%29))
  (Transformation|SetRelativeLocation (Variables|Default|GetMixerFill) (Math|Vector|MakeVector 0.0 0.0 (Math|Interpolation|FInterpTo (.z (Variables|/Script/Engine.SceneComponent|GetRelativeLocation (Variables|Default|GetMixerFill))) (Utilities|Select :Index (Variables|Default|GetFullness) :Option%200 21.0 :Option%201 36.599998 :Option%202 53.299999 :Option%203 7e+01) DeltaSeconds 1e+01)) false false))

(fn ConstructionScript)

(fn AddIngredient
  (params (Flour :type Boolean) (Yeast :type Boolean) (Salt :type Boolean))
  (Utilities|FlowControl|Sequence
    (:then_0
      (if Flour
        (Variables|Default|SetIsFlourLoaded true)))
    (:then_1
      (if Yeast
        (Variables|Default|SetIsYeastLoaded true)))
    (:then_2
      (if Salt
        (Variables|Default|SetIsSaltLoaded true)))
    (:then_3
      (Variables|Default|SetFullness (+ (Math|Conversions|ToInteger(Boolean) (Variables|Default|GetIsFlourLoaded)) (Math|Conversions|ToInteger(Boolean) (Variables|Default|GetIsYeastLoaded)) (Math|Conversions|ToInteger(Boolean) (Variables|Default|GetIsSaltLoaded)))))))