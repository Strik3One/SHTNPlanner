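; BP_DoughTable is a bakery appliance actor that visually shows how much dough is on the table.
; Each tick it eases the Z scale of DoughScale toward one of five levels selected by DoughOnTable, hiding the Dough component when nearly flat.
; SpawnTray spawns a BP_BreadTray at TrayLocation and stores it in Tray; nothing in this Blueprint calls it.
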(event EventBeginPlay)

(event Collision|EventActorBeginOverlap
  (params (OtherActor :type Actor%20Object%20Reference)))

(event EventTick
  (params (DeltaSeconds :type Float%20%28single-precision%29))
  (bind _doughscale (Variables|Default|GetDoughScale))
  (bind _doughontable (Variables|Default|GetDoughOnTable))
  (bind _dough (Variables|Default|GetDough))
  (bind _returnvalue (Rendering|IsVisible _dough))
  (bind _returnvalue_2 (Utilities|Select :Index _doughontable :Option%200 0.0 :Option%201 0.25 :Option%202 0.5 :Option%203 0.75 :Option%204 1.0))
  (bind _relativescale3d (Variables|/Script/Engine.SceneComponent|GetRelativeScale3D _doughscale))
  (bind _returnvalue_3 (Math|Interpolation|FInterpTo (.z _relativescale3d) _returnvalue_2 DeltaSeconds 5.0))
  (Transformation|SetRelativeScale3D (Variables|Default|GetDoughScale) (Math|Vector|MakeVector 1.0 1.0 _returnvalue_3))
  (if (<= _returnvalue_3 0.01)
    (if _returnvalue
      (Rendering|SetVisibility _dough false false))
    (elif (not _returnvalue)
      (Rendering|SetVisibility _dough true false))))

(fn ConstructionScript)

(fn SpawnTray
  (bind _returnvalue (Game|SpawnActorfromClass "/Game/Bakery/BP_BreadTray.BP_BreadTray_C" (Transformation|GetWorldTransform (Variables|Default|GetTrayLocation)) "AlwaysSpawn" 0 0))
  (Variables|Default|SetTray _returnvalue))