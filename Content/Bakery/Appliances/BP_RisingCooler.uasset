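; BP_RisingCooler is a bakery appliance that stores trays in slots tied to four tray location components.
; BeginPlay caches the world locations of those components.
; AddTray puts a tray in the first empty slot and returns that slot's location for placement.
; GetTray finds the first valid tray in a specific TrayState, clears its slot and returns it.
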(event EventBeginPlay
  (Variables|Default|SetTrayLocation (Utilities|Array|MakeArray (Transformation|GetWorldLocation (Variables|Default|GetTrayLocation1)) (Transformation|GetWorldLocation (Variables|Default|GetTrayLocation2)) (Transformation|GetWorldLocation (Variables|Default|GetTrayLocation3)) (Transformation|GetWorldLocation (Variables|Default|GetTrayLocation4)))))

(event Collision|EventActorBeginOverlap
  (params (OtherActor :type Actor%20Object%20Reference)))

(event EventTick
  (params (DeltaSeconds :type Float%20%28single-precision%29)))

(fn ConstructionScript)

(fn AddTray
  (params (Tray :type BP%20Bread%20Tray%20Object%20Reference))
  (for (_array_element _array_index) (Variables|Default|GetTrays)
    (if (== _array_element 0)
      (Utilities|Array|SetArrayElem (Variables|Default|GetTrays) _array_index Tray)
      (return (Utilities|Array|Get(acopy) (Variables|Default|GetTrayLocation) _array_index)))))

(fn GetTray
  (for (_array_element _array_index) (Variables|Default|GetTrays)
    (Utilities|IsValid _array_element
      (:Is%20Valid
        (if (Utilities|Enum|Equal(Enum) (Variables|/Game/Bakery/BP_BreadTray.BP_BreadTray_C|GetTrayState _array_element) "NewEnumerator1")
          (bind _output_get (LocalVariables|SetOutputTray _array_element))
          (Utilities|Array|SetArrayElem (Variables|Default|GetTrays) _array_index 0)
          (return _output_get))))))