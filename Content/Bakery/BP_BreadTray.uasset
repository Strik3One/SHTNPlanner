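; Bakery bread tray that holds up to four loaves and tracks their stage: Dough, Risen or Baked.
; Adding or removing bread toggles loaf mesh visibility and updates the Full flag.
; State changes swap all four meshes, and IncrementState cycles through the stages.
; StartRising stores the baker and starts a timer that sets the tray to Risen and increments a world-state value on that baker.
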(event Custom|StartRising
  (params (Baker :type PC%20Baker%20Controller%20Object%20Reference))
  (Variables|Default|SetBakerController Baker)
  (Utilities|Time|SetTimerbyEvent (delegate Custom|FinishRising) 3e+01))

(event Custom|FinishRising
  (bind _returnvalue (Utilities|Enum|LiteralenumEnum_BakeryWorldState "NewEnumerator3"))
  (bind _bakercontroller (Variables|Default|GetBakerController))
  (CallFunction|SetTrayState "NewEnumerator1")
  (bind _value (Class|SHTNControllerLibrary|GetWorldStateValue _bakercontroller _returnvalue))
  (Class|SHTNControllerLibrary|SetWorldStateasValue _bakercontroller _returnvalue (+ _value 1)))

(event EventBeginPlay)

(event Collision|EventActorBeginOverlap
  (params (OtherActor :type Actor%20Object%20Reference)))

(event EventTick
  (params (DeltaSeconds :type Float%20%28single-precision%29)))

(fn ConstructionScript)

(fn SetTrayState
  (params (NewState :type Enum_BreadStates%20Enum :default "NewEnumerator0"))
  (bind _output_get (Variables|Default|SetTrayState NewState))
  (|SetStaticMeshes _output_get))

(fn AddBread
  (bind _output_get (Variables|Default|SetBreadAmount (Math|Integer|Clamp(Integer) (+ (Variables|Default|GetBreadAmount) 1) 0 4)))
  (if (> _output_get 0)
    (Rendering|SetVisibility (Utilities|Array|Get(acopy) (Utilities|Array|MakeArray (Variables|Default|GetBread1) (Variables|Default|GetBread2) (Variables|Default|GetBread3) (Variables|Default|GetBread4)) (- _output_get 1)) true true)
    (Variables|Default|SetFull (== (Variables|Default|GetBreadAmount) 4))))

(fn RemoveBread
  (bind _output_get (Variables|Default|SetBreadAmount (Math|Integer|Clamp(Integer) (- (Variables|Default|GetBreadAmount) 1) 0 4)))
  (Rendering|SetVisibility (Utilities|Array|Get(acopy) (Utilities|Array|MakeArray (Variables|Default|GetBread4) (Variables|Default|GetBread3) (Variables|Default|GetBread2) (Variables|Default|GetBread1)) _output_get) false true)
  (Variables|Default|SetFull (> (Variables|Default|GetBreadAmount) 0)))

(fn IncrementState
  (CallFunction|SetTrayState (select (Utilities|Enum|Equal(Enum) (Variables|Default|GetTrayState) "NewEnumerator2") "NewEnumerator0" (Utilities|Enum|ByteToEnumEnum_BreadStates (+ (Variables|Default|GetTrayState) 1)))))